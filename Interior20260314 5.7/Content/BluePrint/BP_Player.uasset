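; BP_Player is the player actor that moves in the Y-Z plane and shoots BP_Bullet1.
; Vertical and Horizontal axis inputs write Direction, which Tick scales by MSpeed and delta time for a swept location update.
; Pressing Fire switches on ShotGage to spawn one, two or three bullets at muzzle and fire-position components, then plays a 2D firing sound.
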(event `self.ReceiveBeginPlay`)

(event `self.ReceiveTick`
  (params (DeltaSeconds :type "Float (single-precision)"))
  ;[1 1 1] 이동
  (`self.K2_SetActorLocation` (+ (`self.K2_GetActorLocation`) (* (* (`self.MSpeed`) DeltaSeconds) (`self.direction`))) true))

(event `InputAxis|Vertical`
  (params (AxisValue :type "Float (single-precision)"))
  (bind _output_get (set `self.direction` (`KismetMathLibrary.MakeVector` 0.0 (stale `InputAxis|Horizontal` AxisValue) AxisValue) :!label _label))
  (set `self.direction` _output_get))

(event `InputAxis|Horizontal`
  (params (AxisValue :type "Float (single-precision)"))
  (goto _label))

(event `self.ReceiveEndPlay`
  (params (EndPlayReason :type "EEndPlayReason Enum" :default "Destroyed")))

(event `InputAction|Fire`
  (params (Key :type "Key Structure"))
  (:`Pressed`
    (switch `int` (`self.ShotGage`)
      (:`0`
        (`self.FireBullet`))
      (:`1`
        (`self.FireBullet_2Shot`))
      (:`2`
        (`self.FireBullet_3Shot`)))
    (`GameplayStatics.PlaySound2D` "/Game/StarterContent/Audio/Fire_Sparks01.Fire_Sparks01" 1.0 1.0 0.0 null null)))

(fn `FireBullet`
  (`|SpawnActorFromClass` "/Game/BluePrint/BP_Bullet1.BP_Bullet1_C" (`KismetMathLibrary.Conv_VectorToTransform` (`SceneComponent.K2_GetComponentLocation` (`self.FirePositionThird`))) "AlwaysSpawn" "MultiplyWithRoot" null null))

(fn `FireBullet_2Shot`
  (`|SpawnActorFromClass` "/Game/BluePrint/BP_Bullet1.BP_Bullet1_C" (`KismetMathLibrary.Conv_VectorToTransform` (`SceneComponent.K2_GetComponentLocation` (`self.Muzzle`))) "AlwaysSpawn" "MultiplyWithRoot" null null)
  (`|SpawnActorFromClass` "/Game/BluePrint/BP_Bullet1.BP_Bullet1_C" (`KismetMathLibrary.Conv_VectorToTransform` (`SceneComponent.K2_GetComponentLocation` (`self.FirePositionSecond`))) "Undefined" "MultiplyWithRoot" null null))

(fn `FireBullet_3Shot`
  (`|SpawnActorFromClass` "/Game/BluePrint/BP_Bullet1.BP_Bullet1_C" (`KismetMathLibrary.Conv_VectorToTransform` (`SceneComponent.K2_GetComponentLocation` (`self.Muzzle`))) "AlwaysSpawn" "MultiplyWithRoot" null null)
  (`|SpawnActorFromClass` "/Game/BluePrint/BP_Bullet1.BP_Bullet1_C" (`KismetMathLibrary.Conv_VectorToTransform` (`SceneComponent.K2_GetComponentLocation` (`self.FirePositionSecond`))) "Undefined" "MultiplyWithRoot" null null)
  (`|SpawnActorFromClass` "/Game/BluePrint/BP_Bullet1.BP_Bullet1_C" (`KismetMathLibrary.Conv_VectorToTransform` (`SceneComponent.K2_GetComponentLocation` (`self.FirePositionThird`))) "Undefined" "MultiplyWithRoot" null null))

(fn `UserConstructionScript`)