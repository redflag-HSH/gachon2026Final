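; BP_Item is a falling pickup that raises the player's ShotGage by one when the player pawn overlaps it.
; The pickup is destroyed only when it grants a charge, so it keeps falling if ShotGage is already at its cap of two.
; Tick moves it down the Z axis at Speed with teleporting, unswept moves and destroys it once it is below Line.
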(event `self.ReceiveActorBeginOverlap`
  (params (OtherActor :type "Actor Object Reference"))
  (if (== OtherActor (`GameplayStatics.GetPlayerPawn` 0))
    (bind _asbp_player (cast `/Game/BluePrint/BP_Player` OtherActor))
    (bind _shotgage (`/Game/BluePrint/BP_Player.ShotGage` _asbp_player))
    (if (< _shotgage 2)
      (set `/Game/BluePrint/BP_Player.ShotGage` (+ _shotgage 1) _asbp_player)
      (`self.K2_DestroyActor`))))

(event `self.ReceiveTick`
  (params (DeltaSeconds :type "Float (single-precision)"))
  (bind _z (.z (`self.K2_GetActorLocation`)))
  (if (< _z (`self.Line`))
    (`self.K2_DestroyActor`)
    (else
      (`self.K2_SetActorLocation` (`KismetMathLibrary.MakeVector` (.x (`self.K2_GetActorLocation`)) (.y (`self.K2_GetActorLocation`)) (- _z (* DeltaSeconds (`self.Speed`)))) false true))))

(fn `UserConstructionScript`)