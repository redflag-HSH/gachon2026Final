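; Boss actor that randomly alternates between a waypoint sweep that spawns enemies and a dash toward the player.
; Timer-chained events set each move's target and duration, Tick lerps the position, and patterns return to the start point before looping.
; The sweep spawns a pair of flanking BP_Enemy at each leg.
; Overlaps lower the player's ShotGage or, from bullets, the boss's HP until it is destroyed.
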(event `MoveToTarget`
  (set `self.StartLoc` (`self.K2_GetActorLocation`))
  (set `self.ElapsedTime` 0.0)
  (set `self.isMoving` true))

(event `MoveToA`
  (set `self.MovTarget` (`self.APos`))
  (set `self.MoveDuration` 0.6)
  (`self.MoveToTarget`)
  (`KismetSystemLibrary.K2_SetTimer` null "MoveToB" 0.6)
  (`self.SummonEnemy`))

(event `MoveToB`
  (set `self.MovTarget` (`self.BPos`))
  (set `self.MoveDuration` 1.5)
  (`self.MoveToTarget`)
  (`KismetSystemLibrary.K2_SetTimer` null "MovetoOriginFromBullet" 1.5)
  (`self.SummonEnemy`))

(event `MovetoOriginFromBullet`
  (set `self.MovTarget` (`self.origin`))
  (set `self.MoveDuration` 0.8)
  (`self.MoveToTarget`)
  (`KismetSystemLibrary.K2_SetTimer` null "StartPatternLoop" 0.8)
  (`self.SummonEnemy`))

(event `DashPat`
  (bind _returnvalue (`GameplayStatics.GetPlayerPawn` 0))
  (`/Engine/EditorBlueprintResources/StandardMacros.IsValid` _returnvalue
    (:`Is Valid`
      (set `self.MovTarget` (+ (`self.K2_GetActorLocation`) (* (`KismetMathLibrary.GetForwardVector` (`KismetMathLibrary.FindLookAtRotation` (`self.K2_GetActorLocation`) (`self.K2_GetActorLocation` _returnvalue))) 3000.0)))
      (set `self.MoveDuration` 0.5)
      (`self.MoveToTarget`)
      (`KismetSystemLibrary.K2_SetTimer` null "ReturnToOrigin" 0.5))
    (:`Is Not Valid`
      (`self.StartPatternLoop`))))

(event `SummonEnemy`
  (bind _returnvalue (`|SpawnActorFromClass` "/Game/BluePrint/BP_Enemy.BP_Enemy_C" (`KismetMathLibrary.Conv_VectorToTransform` (+ (`self.K2_GetActorLocation`) (* (`self.GetActorRightVector`) 200.0))) "Undefined" "MultiplyWithRoot" null null))
  (set `/Game/BluePrint/BP_Enemy.Spawner` (`self.spawner`) _returnvalue)
  (bind _returnvalue_2 (`|SpawnActorFromClass` "/Game/BluePrint/BP_Enemy.BP_Enemy_C" (`KismetMathLibrary.Conv_VectorToTransform` (+ (`self.K2_GetActorLocation`) (* (`self.GetActorRightVector`) -200.0))) "Undefined" "MultiplyWithRoot" null null))
  (set `/Game/BluePrint/BP_Enemy.Spawner` (`self.spawner`) _returnvalue_2))

(event `ReturnToOrigin`
  (set `self.MovTarget` (`self.origin`))
  (set `self.MoveDuration` 2.0)
  (`self.MoveToTarget`)
  (`KismetSystemLibrary.K2_SetTimer` null "StartPatternLoop" 2.0))

(event `StartPatternLoop`
  (bind _returnvalue (`KismetMathLibrary.RandomIntegerInRange` 0 1))
  (`KismetSystemLibrary.K2_SetTimerDelegate` (delegate `StartPatternLoop`) 10.0)
  (`KismetSystemLibrary.PrintString` (`KismetStringLibrary.Conv_IntToString` _returnvalue))
  (switch `int` _returnvalue
    (:`0`
      (`self.MoveToA`))
    (:`1`
      (`self.DashPat`))))

(event `self.ReceiveBeginPlay`
  (set `self.origin` (`self.K2_GetActorLocation`))
  (set `self.BossHP` 100)
  (`self.StartPatternLoop`))

(event `self.ReceiveTick`
  (params (DeltaSeconds :type "Float (single-precision)"))
  (bind _returnvalue (/ (`self.ElapsedTime`) (`self.MoveDuration`)))
  (if (`self.isMoving`)
    (set `self.ElapsedTime` (+ (`self.ElapsedTime`) DeltaSeconds))
    (`self.K2_SetActorLocation` (`KismetMathLibrary.VLerp` (`self.StartLoc`) (`self.MovTarget`) _returnvalue))
    (if (>= _returnvalue 1.0)
      (set `self.isMoving` false))))

(event `self.ReceiveActorBeginOverlap`
  (params (OtherActor :type "Actor Object Reference"))
  (bind _asbp_player (cast `/Game/BluePrint/BP_Player` OtherActor)
    (:`then`
      (set `/Game/BluePrint/BP_Player.ShotGage` (- (`/Game/BluePrint/BP_Player.ShotGage` _asbp_player) 1) _asbp_player))
    (:`CastFailed`
      (cast `/Game/BluePrint/BP_Bullet1` OtherActor)
      (set `self.BossHP` (- (`self.BossHP`) 1))
      (if (< (`self.BossHP`) 0)
        (`self.K2_DestroyActor`)))))

(fn `Charge`)

(fn `PatternSelect`)

(fn `UserConstructionScript`)