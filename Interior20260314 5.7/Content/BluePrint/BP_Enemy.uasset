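; BP_Enemy is an enemy that homes in on the player and explodes on its first overlap.
; Each Tick, FindDirection aims at the player, or straight down without a valid target, then the actor moves unswept and faces the player with a pitch offset.
; Overlap destroys it, notifies BP_EnemyManager and plays effects.
; A player hit costs ShotGage or destroys an empty player; other hits may drop BP_Item when ShotGage is low.
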(event `self.ReceiveBeginPlay`
  (set `self.Target` (`GameplayStatics.GetPlayerPawn` 0)))

(event `self.ReceiveTick`
  (params (DeltaSeconds :type "Float (single-precision)"))
  ;[1 1 1] 이동
  (`self.FindDirection`)
  (`self.K2_SetActorLocation` (+ (`self.K2_GetActorLocation`) (* (* (`self.MSpeed`) DeltaSeconds) (`self.direction`))))
  (`self.K2_SetActorRotation` (`KismetMathLibrary.MakeRotator` (.roll (`KismetMathLibrary.FindLookAtRotation` (`self.K2_GetActorLocation`) (`self.K2_GetActorLocation` (`GameplayStatics.GetPlayerPawn` 0)))) (+ (.pitch (`KismetMathLibrary.FindLookAtRotation` (`self.K2_GetActorLocation`) (`self.K2_GetActorLocation` (`GameplayStatics.GetPlayerPawn` 0)))) 90.0) (.yaw (`KismetMathLibrary.FindLookAtRotation` (`self.K2_GetActorLocation`) (`self.K2_GetActorLocation` (`GameplayStatics.GetPlayerPawn` 0)))))))

(event `self.ReceiveEndPlay`
  (params (EndPlayReason :type "EEndPlayReason Enum" :default "Destroyed")))

(event `self.Cube.OnComponentBeginOverlap`
  (params (OverlappedComponent :type "PrimitiveComponent Object Reference") (OtherActor :type "Actor Object Reference") (OtherComp :type "PrimitiveComponent Object Reference") (OtherBodyIndex :type Integer) (bFromSweep :type Boolean) (SweepResult :type "HitResult Structure (by ref)"))
  (`self.K2_DestroyActor`)
  (bind _asbp_enemy_manager (cast `/Game/BluePrint/BP_EnemyManager` (`self.Spawner`)))
  (`/Game/BluePrint/BP_EnemyManager.OnDeath` _asbp_enemy_manager)
  (`GameplayStatics.SpawnEmitterAtLocation` "/Game/StarterContent/Particles/P_Explosion.P_Explosion" (`self.K2_GetActorLocation`))
  (`GameplayStatics.PlaySound2D` "/Game/StarterContent/Audio/Explosion01.Explosion01" 1.0 1.0 0.0 null null)
  (bind _asbp_player (cast `/Game/BluePrint/BP_Player` OtherActor)
    (:`then`
      (if (<= (`/Game/BluePrint/BP_Player.ShotGage` _asbp_player) 0)
        (`self.K2_DestroyActor` _asbp_player)
        (else
          (set `/Game/BluePrint/BP_Player.ShotGage` (- (`/Game/BluePrint/BP_Player.ShotGage` _asbp_player) 1) _asbp_player))))
    (:`CastFailed`
      (bind _asbp_player_2 (cast `/Game/BluePrint/BP_Player` (`GameplayStatics.GetPlayerPawn` 0)))
      (if (< (`/Game/BluePrint/BP_Player.ShotGage` _asbp_player_2) 2)
        (if (`KismetMathLibrary.RandomBool`)
          (`|SpawnActorFromClass` "/Game/BluePrint/BP_Item.BP_Item_C" (`self.GetTransform`) "Undefined" "MultiplyWithRoot" null null))))))

(fn `FindDirection`
  (`/Engine/EditorBlueprintResources/StandardMacros.IsValid` (`self.Target`)
    (:`Is Valid`
      (set `self.direction` (`KismetMathLibrary.Normal` (- (`self.K2_GetActorLocation` (`self.Target`)) (`self.K2_GetActorLocation`)))))
    (:`Is Not Valid`
      (set `self.direction` (0.0 0.0 -1.0)))))

(fn `UserConstructionScript`)