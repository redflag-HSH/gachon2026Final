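; BP_EnemyManager is an enemy spawner that creates BP_Enemy actors on a timer and brings in a single BP_Boss after more than five recorded deaths.
; Tick accumulates delta time, then spawns at fixed X, randomized Y and a Z offset fixed at SpawnRange, since its random bounds are equal.
; Spawns receive the manager as Spawner, OnDeath increments the kill count, and regular spawning continues after the boss appears.
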(event `self.ReceiveTick`
  (params (DeltaSeconds :type "Float (single-precision)"))
  (bind _spawnrange (`self.SpawnRange`))
  (if (> (`self.KilledCount`) 5)
    (if (`self.IsBossSpawned`)
      (bind _output_get (set `self.CreateCount` (+ DeltaSeconds (`self.CreateCount`)) :!label _label))
      (if (>= _output_get (`self.CreateTime`))
        (set `self.CreateCount` 0.0)
        (bind _returnvalue (`|SpawnActorFromClass` "/Game/BluePrint/BP_Enemy.BP_Enemy_C" (`KismetMathLibrary.MakeTransform` (`KismetMathLibrary.MakeVector` -60.0 (+ (.y (`self.K2_GetActorLocation`)) (`KismetMathLibrary.RandomFloatInRange` (* _spawnrange -1.0) _spawnrange)) (+ (.z (`self.K2_GetActorLocation`)) (`KismetMathLibrary.RandomFloatInRange` _spawnrange _spawnrange)))) "Undefined" "MultiplyWithRoot" null null))
        (set `/Game/BluePrint/BP_Enemy.Spawner` self _returnvalue))
      (else
        (bind _returnvalue_2 (`|SpawnActorFromClass` "/Game/BluePrint/BP_Boss.BP_Boss_C" (`KismetMathLibrary.Conv_VectorToTransform` (`self.K2_GetActorLocation`)) "Undefined" "MultiplyWithRoot" null null))
        (set `self.IsBossSpawned` true)
        (set `/Game/BluePrint/BP_Boss.spawner` self _returnvalue_2)))
    (else
      (goto _label))))

(event `OnDeath`
  (set `self.KilledCount` (+ (`self.KilledCount`) 1)))

(fn `UserConstructionScript`)